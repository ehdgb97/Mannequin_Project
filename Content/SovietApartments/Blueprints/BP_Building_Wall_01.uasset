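; BP_Building_Wall_01 is a procedural apartment building wall, assembled in the construction script from floor and segment counts.
; It lays a ground-mesh row, stacks upper floors that cycle through wall variations by segment index, then caps them with a roof row.
; Wall and ground spacing follows mesh bounds, while the roof assumes 300-unit modules.
; Despite the InstancedMesh array name, every piece is a separate StaticMeshComponent.
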(event EventBeginPlay)

(event Collision|EventActorBeginOverlap
  (params (OtherActor :type Actor%20Object%20Reference)))

(event EventTick
  (params (DeltaSeconds :type Float%20%28single-precision%29)))

(fn ConstructionScript
  (bind _groundmesh (Variables|Default|GetGroundMesh))
  (bind _instancedmesh (Variables|Default|GetInstancedMesh))
  (bind _returnvalue (StaticMesh|GetBounds _groundmesh))
  (bind _boxextent (Math|BoxSphereBounds|BreakBoxSphereBounds _returnvalue))
  (bind (_x _y _z) (Math|Vector|BreakVector _boxextent))
  (bind _returnvalue_2 (* _z 2.0))
  (Utilities|FlowControl|Sequence
    (:then_0
      ;[1 1 1] Get number of Wall Variations
      (bind _output_get (Variables|Default|SetNumberOfVariations (Utilities|Array|Length _instancedmesh)))
      ;[1 1 1] Wall
      (for _index (range 0 (- (Variables|Default|GetNumberOfFloors) 1))
        (for _index_2 (range 0 (- (Variables|Default|GetNumberOfSegments) 1))
          (bind _returnvalue_3 (AddComponent|AddStaticMeshComponent false (Math|Transform|MakeTransform (Math|Vector|MakeVector 0.0 (* _index_2 (* (.Y (Math|Vector|BreakVector (.BoxExtent (Math|BoxSphereBounds|BreakBoxSphereBounds (StaticMesh|GetBounds (Utilities|Array|Get(acopy) _instancedmesh (Math|Float|Truncate (.Remainder (Math|Float|Division(WholeandRemainder) (Math|Conversions|ToFloat(Integer) _index_2) (Math|Conversions|ToFloat(Integer) _output_get)))))))))) -2.0)) (+ (* _index (* (.Z (Math|Vector|BreakVector (.BoxExtent (Math|BoxSphereBounds|BreakBoxSphereBounds (StaticMesh|GetBounds (Utilities|Array|Get(acopy) _instancedmesh (Math|Float|Truncate (.Remainder (Math|Float|Division(WholeandRemainder) (Math|Conversions|ToFloat(Integer) _index_2) (Math|Conversions|ToFloat(Integer) _output_get)))))))))) 2.0)) _returnvalue_2)) (Math|Rotator|MakeRotator 0.0 0.0 (* (Math|Conversions|ToFloat(Integer) 0) 9e+01)))))
          (Components|StaticMesh|SetStaticMesh _returnvalue_3 (Utilities|Array|Get(acopy) _instancedmesh (Math|Float|Truncate (.Remainder (Math|Float|Division(WholeandRemainder) (Math|Conversions|ToFloat(Integer) _index_2) (Math|Conversions|ToFloat(Integer) _output_get)))))))))
    (:then_1
      ;[1 1 1] Roof
      (for _index_3 (range 0 (- (Variables|Default|GetNumberOfSegments) 1))
        (bind _returnvalue_4 (AddComponent|AddStaticMeshComponent false (Math|Transform|MakeTransform (Math|Vector|MakeVector 0.0 (* _index_3 -3e+02) (+ (* (Variables|Default|GetNumberOfFloors) 3e+02) _returnvalue_2)))))
        (Components|StaticMesh|SetStaticMesh _returnvalue_4 (Variables|Default|GetRoofMesh))))
    (:then_2
      ;[1 1 1] Ground
      (for _index_4 (range 0 (- (Variables|Default|GetNumberOfSegments) 1))
        (bind _returnvalue_5 (AddComponent|AddStaticMeshComponent false (Math|Transform|MakeTransform (Math|Vector|MakeVector 0.0 (* _index_4 (* _y -2.0)) 0.0))))
        (Components|StaticMesh|SetStaticMesh _returnvalue_5 (Variables|Default|GetGroundMesh))
        (Rendering|Material|SetMaterial _returnvalue_5 0 0)))))