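; BP_LDH is a player character with a camera-aimed air dash and an aim widget added to the screen on BeginPlay.
; Holding Left Shift while falling slows global time; releasing it in the air restores time and dashes, gated by paired DoOnce nodes re-armed on jump.
; AirDash chains two timed camera-forward launches, then Firction zeroes velocity to stop the character.
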(event EventBeginPlay
  (bind _returnvalue (UserInterface|CreateWidget "/Game/ALDH/BP_Aim.BP_Aim_C"))
  (UserInterface|Viewport|AddtoViewport _returnvalue 0))

(event Collision|EventActorBeginOverlap
  (params (OtherActor :type Actor%20Object%20Reference)))

(event EventTick
  (params (DeltaSeconds :type Float%20%28single-precision%29)))

(event EventOnJumped
  (Utilities|FlowControl|DoOnce false) ; enters at Reset
)

(event Input|KeyboardEvents|LeftShift
  (params (Key :type Key%20Structure :default "None"))
  (bind _charactermovement (Variables|Character|GetCharacterMovement))
  (bind _returnvalue (AI|Components|NavMovement|IsFalling _charactermovement))
  (:Pressed
    (if _returnvalue
      (Utilities|FlowControl|DoOnce false
        (:Completed
          (Utilities|Time|SetGlobalTimeDilation 0.1)
          (goto _label Reset)))))
  (:Released
    (if _returnvalue
      (Utilities|FlowControl|DoOnce false :!label _label
        (:Completed
          (Utilities|Time|SetGlobalTimeDilation 1.0)
          (Utilities|AirDash))))))

(event Input|MouseEvents|RightMouseButton
  (params (Key :type Key%20Structure :default "None")))

(fn ConstructionScript)

(fn Firction
  (Variables|/Script/Engine.MovementComponent|SetVelocity (Variables|Character|GetCharacterMovement) "0, 0, 0"))