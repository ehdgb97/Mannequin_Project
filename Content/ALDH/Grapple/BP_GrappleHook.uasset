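; BP_GrappleHook is a grapple hook projectile that flies toward a Target actor and locks in place on arrival.
; BeginPlay caches start and end locations and launches ProjectileMovement along their direction at Speed.
; Tick compares squared distances from the start for hook and Target, then snaps the hook to the cached end and zeroes velocity.
; DistanceToTarget returns the remaining distance to that cached end.
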(event EventBeginPlay
  ;[1 1 1] Comment
  (Variables|Private|SetStartingLocation (Transformation|GetActorLocation))
  (Variables|Private|SetEndingLocation (Transformation|GetActorLocation (Variables|Default|GetTarget)))
  (Variables|Private|SetDirection (Math|Vector|Normalize (- (Variables|Private|GetEndingLocation) (Variables|Private|GetStartingLocation))))
  (Variables|/Script/Engine.MovementComponent|SetVelocity (Variables|Default|GetProjectileMovement) (* (Variables|Private|GetDirection) (Variables|Default|GetSpeed))))

(event EventTick
  (params (DeltaSeconds :type Float%20%28single-precision%29))
  ;[1 1 1] 출발하여 특정 타겟과 거리가 가까워지면 위치가 고정된다.
  (if (>= (Class|KismetMathLibrary|VectorDistanceSquared (Transformation|GetActorLocation) (Variables|Private|GetStartingLocation)) (Class|KismetMathLibrary|VectorDistanceSquared (Transformation|GetActorLocation (Variables|Default|GetTarget)) (Variables|Private|GetStartingLocation)))
    (Transformation|SetActorLocation (+ (Variables|Private|GetStartingLocation) (* (Variables|Private|GetDirection) (Math|Vector|Distance(Vector) (Variables|Private|GetStartingLocation) (Variables|Private|GetEndingLocation)))) false false)
    (Variables|/Script/Engine.MovementComponent|SetVelocity (Variables|Default|GetProjectileMovement) "0, 0, 0")))

(fn ConstructionScript)

(fn DistancetoTarget
  (return (Math|Vector|Distance(Vector) (Variables|Private|GetEndingLocation) (Transformation|GetActorLocation))))