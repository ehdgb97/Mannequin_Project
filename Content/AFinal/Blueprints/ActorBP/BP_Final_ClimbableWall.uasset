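; BP_Final_ClimbableWall is a wall actor that lets BP_Final_Player climb while inside its box collision.
; Overlap begin sets the player's CanClimbing flag.
; Overlap end clears both climbing flags, launches the player backward along its forward vector and restores orient-rotation-to-movement, whether or not it was climbing.
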(event OnComponentBeginOverlap(BoxCollision)
  (params (OverlappedComponent :type Primitive%20Component%20Object%20Reference) (OtherActor :type Actor%20Object%20Reference) (OtherComp :type Primitive%20Component%20Object%20Reference) (OtherBodyIndex :type Integer) (bFromSweep :type Boolean) (SweepResult :type Hit%20Result%20Structure%20%28by%20ref%29))
  (bind _asbp_final_player (Utilities|Casting|CastToBP_Final_Player OtherActor))
  (Variables|/Game/AFinal/Blueprints/BP_Final_Player.BP_Final_Player_C|SetcanClimbing? _asbp_final_player true))

(event OnComponentEndOverlap(BoxCollision)
  (params (OverlappedComponent :type Primitive%20Component%20Object%20Reference) (OtherActor :type Actor%20Object%20Reference) (OtherComp :type Primitive%20Component%20Object%20Reference) (OtherBodyIndex :type Integer))
  (bind _asbp_final_player (Utilities|Casting|CastToBP_Final_Player OtherActor))
  (if (Variables|/Game/AFinal/Blueprints/BP_Final_Player.BP_Final_Player_C|GetisClimbing? _asbp_final_player)
    _
    (else
      _))
  (Variables|/Game/AFinal/Blueprints/BP_Final_Player.BP_Final_Player_C|SetcanClimbing? _asbp_final_player false)
  (Variables|/Game/AFinal/Blueprints/BP_Final_Player.BP_Final_Player_C|SetisClimbing? _asbp_final_player false)
  (Character|LaunchCharacter _asbp_final_player (Math|Vector|MakeVector (.x (* (Transformation|GetActorForwardVector _asbp_final_player) -2e+02)) (.y (* (Transformation|GetActorForwardVector _asbp_final_player) -2e+02)) 0.0) false false)
  (Variables|/Script/Engine.CharacterMovementComponent|SetbOrientRotationToMovement (Variables|/Script/Engine.Character|GetCharacterMovement _asbp_final_player) true))

(fn ConstructionScript)