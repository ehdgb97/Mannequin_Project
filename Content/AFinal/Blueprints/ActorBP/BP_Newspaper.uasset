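; BP_Newspaper is an interactable newspaper actor that shows a readable newspaper widget while E is held.
; Its Box overlap enables input and sets an in-range flag, before any player cast, so any overlapping actor sets it.
; The News1 actor tag selects WBP_Newspaper1, otherwise WBP_Newspaper2 is shown.
; Releasing E or the player leaving the box removes the visible widget; input is never disabled.
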(event OnComponentBeginOverlap(Box)
  (params (OverlappedComponent :type Primitive%20Component%20Object%20Reference) (OtherActor :type Actor%20Object%20Reference) (OtherComp :type Primitive%20Component%20Object%20Reference) (OtherBodyIndex :type Integer) (bFromSweep :type Boolean) (SweepResult :type Hit%20Result%20Structure%20%28by%20ref%29))
  (Input|EnableInput (Game|GetPlayerController 0))
  (Variables|Default|SetplayerAtNewspaper? true)
  (Utilities|Casting|CastToBP_Final_Player OtherActor))

(event OnComponentEndOverlap(Box)
  (params (OverlappedComponent :type Primitive%20Component%20Object%20Reference) (OtherActor :type Actor%20Object%20Reference) (OtherComp :type Primitive%20Component%20Object%20Reference) (OtherBodyIndex :type Integer))
  (Variables|Default|SetplayerAtNewspaper? false)
  (Utilities|Casting|CastToBP_Final_Player OtherActor)
  (Utilities|FlowControl|Sequence
    (:then_0
      (if (Variables|Default|GetisVIsibleNews1?)
        (Widget|RemovefromParent (stale Input|KeyboardEvents|E _returnvalue))
        (Variables|Default|SetisVIsibleNews1? false)))
    (:then_1
      (if (Variables|Default|GetisVisibleNews2?)
        (Widget|RemovefromParent (stale Input|KeyboardEvents|E _returnvalue_2))
        (Variables|Default|SetisVisibleNews2? false)))))

(event EventTick
  (params (DeltaSeconds :type Float%20%28single-precision%29)))

(event Input|KeyboardEvents|E
  (params (Key :type Key%20Structure))
  (:Pressed
    (if (Variables|Default|GetplayerAtNewspaper?)
      (if (Actor|ActorHasTag "News1")
        (bind _returnvalue (UserInterface|CreateWidget "/Game/AFinal/Ui/WBP_Newspaper1.WBP_Newspaper1_C"))
        (UserInterface|Viewport|AddtoViewport _returnvalue 0)
        (Variables|Default|SetisVIsibleNews1? true)
        (else
          (bind _returnvalue_2 (UserInterface|CreateWidget "/Game/AFinal/Ui/WBP_Newspaper2.WBP_Newspaper2_C"))
          (UserInterface|Viewport|AddtoViewport _returnvalue_2 0)
          (Variables|Default|SetisVisibleNews2? true)))
      (else
        (Variables|Default|SetisVIsibleNews1? false)
        (Variables|Default|SetisVisibleNews2? false))))
  (:Released
    (Utilities|FlowControl|Sequence
      (:then_0
        (if (Variables|Default|GetisVIsibleNews1?)
          (Widget|RemovefromParent _returnvalue)
          (Variables|Default|SetisVIsibleNews1? false)))
      (:then_1
        (if (Variables|Default|GetisVisibleNews2?)
          (Widget|RemovefromParent _returnvalue_2)
          (Variables|Default|SetisVisibleNews2? false))))))

(fn ConstructionScript)