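; A movable cube that BP_FinalPlayer can push.
; Two overlap volumes, one for the X axis and one for Y, enable physics simulation on the cube and set the player's IsPushing flag when the player enters.
; Leaving either volume clears IsPushing, but only the Y volume turns physics back off; leaving the X volume keeps the cube simulating.
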(event OnComponentBeginOverlap(YAxisCollision)
  (params (OverlappedComponent :type Primitive%20Component%20Object%20Reference) (OtherActor :type Actor%20Object%20Reference) (OtherComp :type Primitive%20Component%20Object%20Reference) (OtherBodyIndex :type Integer) (bFromSweep :type Boolean) (SweepResult :type Hit%20Result%20Structure%20%28by%20ref%29))
  ;[1 1 1] Y Axis Collision
  (bind _asbp_jyp_player (Utilities|Casting|CastToBP_FinalPlayer OtherActor))
  (Physics|SetSimulatePhysics (Variables|Default|GetCube) true)
  (Variables|/Game/AFinal/Blueprints/BP_FinalPlayer.BP_FinalPlayer_C|SetIsPushing? _asbp_jyp_player true))

(event OnComponentEndOverlap(YAxisCollision)
  (params (OverlappedComponent :type Primitive%20Component%20Object%20Reference) (OtherActor :type Actor%20Object%20Reference) (OtherComp :type Primitive%20Component%20Object%20Reference) (OtherBodyIndex :type Integer))
  ;[1 1 1] Y Axis Collision
  (bind _asbp_jyp_player (Utilities|Casting|CastToBP_FinalPlayer OtherActor))
  (Physics|SetSimulatePhysics (Variables|Default|GetCube) false)
  (Variables|/Game/AFinal/Blueprints/BP_FinalPlayer.BP_FinalPlayer_C|SetIsPushing? _asbp_jyp_player false))

(event OnComponentBeginOverlap(XAxisCollision)
  (params (OverlappedComponent :type Primitive%20Component%20Object%20Reference) (OtherActor :type Actor%20Object%20Reference) (OtherComp :type Primitive%20Component%20Object%20Reference) (OtherBodyIndex :type Integer) (bFromSweep :type Boolean) (SweepResult :type Hit%20Result%20Structure%20%28by%20ref%29))
  ;[1 1 1] X Axis Collision
  (bind _asbp_jyp_player (Utilities|Casting|CastToBP_FinalPlayer OtherActor))
  (Physics|SetSimulatePhysics (Variables|Default|GetCube) true)
  (Variables|/Game/AFinal/Blueprints/BP_FinalPlayer.BP_FinalPlayer_C|SetIsPushing? _asbp_jyp_player true))

(event OnComponentEndOverlap(XAxisCollision)
  (params (OverlappedComponent :type Primitive%20Component%20Object%20Reference) (OtherActor :type Actor%20Object%20Reference) (OtherComp :type Primitive%20Component%20Object%20Reference) (OtherBodyIndex :type Integer))
  ;[1 1 1] X Axis Collision
  (bind _asbp_jyp_player (Utilities|Casting|CastToBP_FinalPlayer OtherActor))
  (Physics|SetSimulatePhysics (Variables|Default|GetCube) true)
  (Variables|/Game/AFinal/Blueprints/BP_FinalPlayer.BP_FinalPlayer_C|SetIsPushing? _asbp_jyp_player false))

(fn ConstructionScript)