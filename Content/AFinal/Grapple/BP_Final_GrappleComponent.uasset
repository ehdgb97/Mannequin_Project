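; Grappling hook component for BP_FinalChar that pulls the player toward grapple target actors.
; Tick runs a four-state machine: Retracted, Firing, Nearing Target (small hop), On Target (velocity pull, then exit launch).
; While retracted and landed, a sphere overlap and line-of-sight traces highlight the target closest to the camera's forward vector.
; AttemptGrapple spawns the hook and a hand-attached cable line, turns the character and starts Firing.
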(event EventBeginPlay
  (bind _asbp_final_char (Utilities|Casting|CastToBP_FinalChar (Components|GetOwner)))
  (Variables|Private|SetOwningCharacter _asbp_final_char))

(event EventTick
  (params (DeltaSeconds :type Float%20%28single-precision%29))
  (switch Utilities|FlowControl|Switch|SwitchonFinal_EGrappleState (Variables|Private|GetGrappleState)
    (:NewEnumerator0
      (Variables|Default|SetGrappleUsing false)
      (if (Variables|/Game/AFinal/Blueprints/BP_FinalChar.BP_FinalChar_C|GetLanded (Variables|Private|GetOwningCharacter))
        (Private|TickRetracted)
        ;[1 1 1] Widget
        (bind _returnvalue (Actor|GetActorOfClass "/Game/AFinal/Blueprints/BP_FinalChar.BP_FinalChar_C"))
        (Widget|SetVisibility (Variables|/Game/ALDH/Ui/WB_Test.WB_Test_C|GetEditableTextBox_2 (Variables|/Game/AFinal/Blueprints/BP_FinalChar.BP_FinalChar_C|GetSkillWidget _returnvalue)) "Visible")))
    (:NewEnumerator1
      (Variables|Default|SetGrappleUsing true)
      (Private|TickFiring)
      (Default|SetActive (Variables|Private|GetCurrentTarget) false)
      (bind _returnvalue_2 (Actor|GetActorOfClass "/Game/AFinal/Blueprints/BP_FinalChar.BP_FinalChar_C"))
      (Widget|SetVisibility (Variables|/Game/ALDH/Ui/WB_Test.WB_Test_C|GetEditableTextBox_2 (Variables|/Game/AFinal/Blueprints/BP_FinalChar.BP_FinalChar_C|GetSkillWidget _returnvalue_2)) "Hidden"))
    (:NewEnumerator2
      (Private|TickNearingTarget))
    (:NewEnumerator3
      (Private|TickonTarget)
      (Default|EventonGrapple (Variables|Private|GetOwningCharacter)))))

(fn TickRetracted
  (bind _returnvalue (Actor|GetActorOfClass "/Game/AFinal/Grapple/BP_Final_GrappleTarget.BP_Final_GrappleTarget_C"))
  (bind _outactors (Collision|SphereOverlapActors (Transformation|GetActorLocation (Variables|Private|GetOwningCharacter)) (Variables|/Game/AFinal/Grapple/BP_Final_GrappleTarget.BP_Final_GrappleTarget_C|GetMax _returnvalue) (Utilities|Array|MakeArray "ObjectTypeQuery1") "/Game/AFinal/Grapple/BP_Final_GrappleTarget.BP_Final_GrappleTarget_C"))
  ;[1 1 1] 여러 타겟들 중에서 이동하기 적합한 타겟을 찾아서 이동가능 타겟으로 설정한다.
  (bind _target (Private|FindBestTarget _outactors))
  (Private|SetCurrentTarget (.AsBP%20Final%20Grapple%20Target (Utilities|Casting|CastToBP_Final_GrappleTarget _target))))

(fn TickFiring
  (if (< (Default|DistancetoTarget (Variables|Private|GetGrappleHook)) (Variables|Private|Constants|GetStartJumpDistance))
    (Character|LaunchCharacter (Variables|Private|GetOwningCharacter) "0, 0,50.000000" true true)
    (Variables|Private|SetGrappleState "NewEnumerator2")))

(fn TickNearingTarget
  (if (<= (.z (Transformation|GetVelocity (Variables|Private|GetOwningCharacter))) 0.0)
    (Variables|Private|SetInitalDirection (Utilities|OwnertoTarget))
    (Variables|Private|SetGrappleState "NewEnumerator3")))

(fn TickonTarget
  (bind _initaldirection (Variables|Private|GetInitalDirection))
  (bind _returnvalue (Math|Vector|MakeVector (.x _initaldirection) (.y _initaldirection) 0.0))
  (bind _returnvalue_2 (Math|Vector|Normalize _returnvalue))
  (bind _returnvalue_3 (* _returnvalue_2 6e+02))
  ;[1 1 1] 타겟과 플레이어의 거리 조건
  (if (< (Transformation|GetDistanceTo (Variables|Private|GetOwningCharacter) (Variables|Private|GetCurrentTarget)) (Variables|Private|Constants|GetEndJumpDistance))
    (Character|LaunchCharacter (Variables|Private|GetOwningCharacter) (Math|Vector|MakeVector (.x _returnvalue_3) (.y _returnvalue_3) 2e+02) true true)
    (Private|SetCurrentTarget)
    (Actor|DestroyActor (Variables|Private|GetGrappleLine))
    (Variables|Private|SetGrappleHook 0)
    (Variables|Private|SetGrappleState "NewEnumerator0")
    (else
      (Variables|/Script/Engine.MovementComponent|SetVelocity (Pawn|GetMovementComponent (Variables|Private|GetOwningCharacter)) (* (Utilities|OwnertoTarget) (Variables|Private|Constants|GetCharacterGrapplespeed))))))

(fn FindBestTarget
  (params (Targets :type Array%20of%20Actor%20Object%20References))
  (bind _owningcharacter (Variables|Private|GetOwningCharacter))
  (for _array_element Targets
    (LocalVariables|SetCurrentTarget%28Local%29 _array_element)
    (bind (_outhit _returnvalue) (Collision|LineTraceByChannel (Transformation|GetActorLocation (Variables|Private|GetOwningCharacter)) (Transformation|GetActorLocation (LocalVariables|GetCurrentTarget%28Local%29)) "TraceTypeQuery1" false (Utilities|Array|MakeArray (Variables|Private|GetOwningCharacter)) "None" true "(R=1.000000,G=0.000000,B=0.000000,A=1.000000)" "(R=0.000000,G=1.000000,B=0.000000,A=1.000000)" 0.3))
    (if _returnvalue
      (if (== (.HitActor (Collision|BreakHitResult _outhit)) (LocalVariables|GetCurrentTarget%28Local%29))
        (Utilities|FlowControl|Sequence
          (:then_0
            ;[1 1 1] Step 1)Calculate the angle to the target
            (LocalVariables|SetCurrent%20Angle%28Local%29 (Class|KismetMathLibrary|DegAcos (Math|Vector|DotProduct (Math|Vector|Normalize (- (Transformation|GetActorLocation (LocalVariables|GetCurrentTarget%28Local%29)) (Transformation|GetActorLocation _owningcharacter))) (Math|Vector|GetForwardVector (Variables|/Game/AFinal/Blueprints/BP_FinalChar.BP_FinalChar_C|GetFollowCamera _owningcharacter))))))
          (:then_1
            ;[1 1 1] Step2) If the angle is less than our current angle make this our new target
            (if (or (< (LocalVariables|GetCurrent%20Angle%28Local%29) (LocalVariables|GetBestAngle%28Local%29)) (not (Utilities|IsValid (LocalVariables|GetBestTarget%28Local%29))))
              (LocalVariables|SetBestTarget%28Local%29 (LocalVariables|GetCurrentTarget%28Local%29))
              (LocalVariables|SetBestAngle%28Local%29 (LocalVariables|GetCurrent%20Angle%28Local%29))))))))
  (return (LocalVariables|GetBestTarget%28Local%29)))

(fn SetCurrentTarget
  (params (NewTarget :type BP%20Final%20Grapple%20Target%20Object%20Reference))
  (if (!= NewTarget (Variables|Private|GetCurrentTarget))
    (Utilities|FlowControl|Sequence
      (:then_0
        (bind _currenttarget (Variables|Private|GetCurrentTarget)
          (:then
            (Default|SetActive _currenttarget false))
          (:else)))
      (:then_1
        (Variables|Private|SetCurrentTarget NewTarget))
      (:then_2
        (bind _currenttarget_2 (Variables|Private|GetCurrentTarget)
          (:then
            (Default|SetActive _currenttarget_2 true))
          (:else))))))

(fn AttemptGrapple
  (switch Utilities|FlowControl|Switch|SwitchonFinal_EGrappleState (Variables|Private|GetGrappleState)
    (:NewEnumerator0
      (bind _currenttarget (Variables|Private|GetCurrentTarget)
        (:then
          (bind _returnvalue (Game|SpawnActorfromClass "/Game/AFinal/Grapple/BP_Final_GrappleHook.BP_Final_GrappleHook_C" (Math|Transform|MakeTransform (Utilities|OwnerLocation) "0, 0, 0" "1,1,1") "AlwaysSpawn" 0 _currenttarget 5e+03 0))
          (Variables|Private|SetGrappleHook _returnvalue)
          (bind _returnvalue_2 (Game|SpawnActorfromClass "/Game/AFinal/Grapple/BP_Final_GrappleLine.BP_Final_GrappleLine_C" (Math|Transform|MakeTransform (Utilities|OwnerLocation) "0, 0, 0" "1,1,1") "Undefined" 0 0))
          (bind _output_get (Variables|Private|SetGrappleLine _returnvalue_2))
          (Transformation|AttachComponentToComponent _output_get (Variables|/Script/Engine.Character|GetMesh (Variables|Private|GetOwningCharacter)) "hand_r" "SnapToTarget" "SnapToTarget" "SnapToTarget" true)
          (Class|CableComponent|SetAttachEndto (Variables|/Script/CableComponent.CableActor|GetCableComponent (Variables|Private|GetGrappleLine)) (Variables|Private|GetGrappleHook) "DefaultSceneRoot" "None")
          ;[1 1 1] Look at Target
          ; 필요한가 생각하기
          (Transformation|SetActorRotation (Variables|Private|GetOwningCharacter) (Math|Rotator|MakeRotfromZX (Math|Vector|MakeVector 0.0 0.0 1.0) (Utilities|OwnertoTarget)))
          (Variables|Private|SetGrappleState "NewEnumerator1"))
        (:else)))))